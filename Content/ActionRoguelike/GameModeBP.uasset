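; Game mode Blueprint for an action roguelike that drives alert-level music and reacts to AI nearly detecting a character.
; Alert-level changes, plus an initial call on BeginPlay, switch between cached 2D soundtracks for None and Caution.
; It binds to every SAIController present at BeginPlay; when a non-Spidey character is about to be detected, Spidey distracts that enemy and the player controller shows the spider minimap.
; A minimap widget notification chain is left disconnected.
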(event `self.ReceiveBeginPlay`
  (add `self.OnAlertLevelChanged` (delegate `OnAlertLevelChanged_Event_0`))
  (bind _returnvalue (`self.GetGameAlertLevel`))
  (`self.OnAlertLevelChanged_Event_0` self _returnvalue)
  (bind _outactors (`GameplayStatics.GetAllActorsOfClass` "/Script/ActionRoguelike.SAIController"))
  (for _array_element _outactors
    (add `SAIController.OnCharacterAboutToBeDetected` _array_element (delegate `OnCharacterAboutToBeDetected`))))

(event `OnCharacterAboutToBeDetected`
  (params (EnemyController :type "SAIController Object Reference") (Character :type "SCharacter Object Reference"))
  (cast `/Game/ActionRoguelike/Companion_AI/Spidey` Character
    (:`then`
      (`KismetSystemLibrary.PrintString` "Spidey About To Be Detected"))
    (:`CastFailed`
      (`KismetSystemLibrary.PrintString` "Player About To Be Detected")
      (bind _returnvalue (`GameplayStatics.GetActorOfClass` "/Game/ActionRoguelike/Companion_AI/Spidey.Spidey_C"))
      (if (`KismetSystemLibrary.IsValid` _returnvalue)
        (`SCharacter.Distract` _returnvalue EnemyController)
        (bind _asplayer_controller_bp (cast `/Game/ActionRoguelike/PlayerControllerBP` (`GameplayStatics.GetPlayerController` 0)))
        (`/Game/ActionRoguelike/PlayerControllerBP.Show Spider MiniMap` _asplayer_controller_bp)))))

(event `OnAlertLevelChanged_Event_0` :!signature `self.OnAlertLevelChanged`
  (params (GameModeBase :type "SGameModeBase Object Reference") (GameAlertLevel :type "AlertLevel Enum" :default "None"))
  (switch `AlertLevel` GameAlertLevel
    (:`None`
      (`self.Play No Alert Soundtrack`))
    (:`Caution`
      (`self.Play Caution Soundtrack`))))

(event `Play Caution Soundtrack`
  (bind _cautionsound (`self.CautionSound`))
  (`self.Stop Soundtrack` (`self.NoAlertSound`))
  (if (`KismetSystemLibrary.IsValid` _cautionsound)
    (`AudioComponent.Play` _cautionsound 0.0)
    (else
      (bind _returnvalue (`GameplayStatics.SpawnSound2D` "/Game/ActionRoguelike/CautionSound.CautionSound" 0.3 1.0 0.0 null false false))
      (set `self.CautionSound` _returnvalue))))

(event `Play No Alert Soundtrack`
  (bind _noalertsound (`self.NoAlertSound`))
  (`self.Stop Soundtrack` (`self.CautionSound`))
  (if (`KismetSystemLibrary.IsValid` _noalertsound)
    (`AudioComponent.Play` _noalertsound 0.0)
    (else
      (bind _returnvalue (`GameplayStatics.SpawnSound2D` "/Game/SFX/Background/Day_Of_Recon.Day_Of_Recon" 0.3 1.0 0.0 null false false))
      (set `self.NoAlertSound` _returnvalue))))

(event `Stop Soundtrack`
  (params (Soundtrack :type "AudioComponent Object Reference (by ref)"))
  (if (`KismetSystemLibrary.IsValid` Soundtrack)
    (`AudioComponent.Stop` Soundtrack)))

(fn `UserConstructionScript`)