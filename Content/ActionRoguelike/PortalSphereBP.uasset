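; PortalSphereBP is a level exit portal that lets the player through only when accompanied by the Spidey companion.
; On overlap by PlayerCharacter, it finds the Spidey actor and opens Success_Exit if the companion is within a short distance of the player.
; Otherwise it prints whether the companion is missing or too far away.
; A ShowMessage helper builds a colored, timed Message_Widget on screen, but the overlap logic does not call it.
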(event `self.ReceiveActorBeginOverlap`
  (params (OtherActor :type "Actor Object Reference"))
  (bind _asplayer_character (cast `/Game/ActionRoguelike/PlayerCharacter` OtherActor))
  (bind _returnvalue (`GameplayStatics.GetActorOfClass` "/Game/ActionRoguelike/Companion_AI/Spidey.Spidey_C"))
  (`/Engine/EditorBlueprintResources/StandardMacros.IsValid` _returnvalue
    (:`Is Valid`
      (if (< (`self.GetDistanceTo` _returnvalue _asplayer_character) 100.0)
        (`GameplayStatics.OpenLevel` "Success_Exit")
        (else
          (`KismetSystemLibrary.PrintString` "Companion is too far away"))))
    (:`Is Not Valid`
      (`KismetSystemLibrary.PrintString` "Cannot pass without companion"))))

(fn `Show Message`
  (params (Message :type String :default "Sample Message") (Color :type "LinearColor Structure") (TimeOnScreen :type "Float (double-precision)" :default 5.0))
  (bind _returnvalue (`|CreateWidget` "/Game/ActionRoguelike/UI/Message_Widget.Message_Widget_C"))
  (set `/Game/ActionRoguelike/UI/Message_Widget.Message` Message _returnvalue)
  (set `/Game/ActionRoguelike/UI/Message_Widget.TimeOnScreen` TimeOnScreen _returnvalue)
  (bind _structout (setmembers `SlateColor` :`StructRef` (make `SlateColor` Color)))
  (set `/Game/ActionRoguelike/UI/Message_Widget.Color` _structout _returnvalue)
  (`UserWidget.AddToViewport` _returnvalue 0))

(fn `UserConstructionScript`)