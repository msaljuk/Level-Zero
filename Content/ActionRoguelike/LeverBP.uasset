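; Interactable lever that grants or removes the KeyCard gameplay tag on the pawn using it.
; Interact flips HandleMesh between two tilted rotations, using its current rotation as the on/off state instead of a separate variable.
; Each flip directly edits ActiveGameplayTags on the instigator's SActionComponent, so the tag change follows the lever's state, not whether that pawn already has the tag.
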(event `SGameplayInterface.Interact`
  (params (InstigatorPawn :type "Pawn Object Reference"))
  (bind _handlemesh (`self.HandleMesh`))
  (bind _keycard (`self.KeyCard`))
  (bind _activegameplaytags (`SActionComponent.ActiveGameplayTags` (`self.GetComponentByClass` InstigatorPawn "/Script/ActionRoguelike.SActionComponent")))
  (if (== (`SceneComponent.RelativeRotation` (`self.HandleMesh`)) (struct :`Pitch` -30.0))
    (`SceneComponent.K2_SetRelativeRotation` _handlemesh (struct :`Pitch` 30.0) false false)
    (`BlueprintGameplayTagLibrary.AddGameplayTag` _activegameplaytags _keycard)
    (else
      (`SceneComponent.K2_SetRelativeRotation` _handlemesh (struct :`Pitch` -30.0) false false)
      (`BlueprintGameplayTagLibrary.RemoveGameplayTag` _activegameplaytags _keycard))))

(fn `UserConstructionScript`)