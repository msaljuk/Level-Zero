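; Ranged minion AI character that reacts to damage and noise.
; Health loss from its attribute component spawns a damage number widget attached to the minion, showing the absolute amount lost.
; Pawn sensing hearing, ignoring its own noise, writes the heard location and time into its MinionControllerBP.
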(event `self.AttributeComp.OnHealthChanged`
  (params (InstigatorActor :type "Actor Object Reference") (OwningComp :type "SAtttributeComponent Object Reference") (NewHealth :type "Float (single-precision)") (Delta :type "Float (single-precision)"))
  (if (< Delta 0.0)
    (bind _returnvalue (`|CreateWidget` "/Game/ActionRoguelike/UI/DamageHealth_Widget.DamageHealth_Widget_C" null self (`KismetMathLibrary.Abs` Delta)))
    (`UserWidget.AddToViewport` _returnvalue 0)))

(event `self.PawnSensingComp.OnHearNoise`
  (params (Instigator :type "Pawn Object Reference") (Location :type "Vector Structure (by ref)") (Volume :type "Float (single-precision)"))
  (if (!= Instigator self)
    (bind _asminion_controller_bp (cast `/Game/ActionRoguelike/AI/MinionControllerBP` (`self.GetController`)))
    (set `SAIController.HeardPlayerLocation` Location _asminion_controller_bp)
    (set `SAIController.LastHeardTime` (`KismetSystemLibrary.GetGameTimeInSeconds`) _asminion_controller_bp)))

(fn `UserConstructionScript`)